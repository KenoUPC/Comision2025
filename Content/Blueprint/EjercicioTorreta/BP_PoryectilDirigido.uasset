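; BP_PoryectilDirigido is a homing projectile from a turret exercise that steers toward a Target actor after a short launch phase.
; It flies straight along its local forward axis until a BeginPlay delay sets Seguir.
; Tick then snaps its rotation to face the Target and moves it by Direccion times Velocidad in local space.
; Movement is per frame without delta-time scaling or sweep, and no hit logic is implemented.
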(event `self.ReceiveBeginPlay`
  (`KismetSystemLibrary.Delay` 2.0)
  (set `self.bSeguir?` true))

(event `self.ReceiveTick`
  (params (DeltaSeconds :type "Float (single-precision)"))
  (if (`self.bSeguir?`)
    (`self.K2_SetActorRotation` (`KismetMathLibrary.FindLookAtRotation` (`self.K2_GetActorLocation`) (`self.K2_GetActorLocation` (`self.Target`))))
    (`self.K2_AddActorLocalOffset` (* (`self.Direccion`) (`self.Velocidad`)))
    (else
      (`self.K2_AddActorLocalOffset` (5.0 0.0 0.0)))))

(fn `UserConstructionScript`)