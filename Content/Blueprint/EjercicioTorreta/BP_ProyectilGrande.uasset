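; Large projectile for a turret exercise that breaks into a burst of smaller projectiles targeted at the player.
; Tick moves it by a local offset each frame, without sweep or delta-time scaling.
; BeginPlay caches the player's BP_Character, waits, then starts a looping timer that spawns BP_PoryectilDirigido shards with that character as target.
; A counter caps the burst, after which the projectile destroys itself.
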(event `self.ReceiveBeginPlay`
  (bind _asbp_character (cast `/Game/Character/BP_Character` (`GameplayStatics.GetPlayerCharacter` 0)))
  (bind _output_get (set `self.As BP Character` _asbp_character))
  (`/Engine/EditorBlueprintResources/StandardMacros.IsValid` _output_get
    (:`Is Valid`
      (`KismetSystemLibrary.Delay` 5.0)
      (`KismetSystemLibrary.K2_SetTimerDelegate` (delegate `DispararEsquirlas`) 0.1 true))))

(event `DispararEsquirlas`
  (if (<= (`self.Contador`) 4)
    (bind _result (`/Engine/EditorBlueprintResources/StandardMacros.IncrementInt` (`self.Contador`))
      (:`  `
        (set `self.Contador` _result)
        (`|SpawnActorFromClass` "/Game/Blueprint/EjercicioTorreta/BP_PoryectilDirigido.BP_PoryectilDirigido_C" (`self.GetTransform`) "Undefined" "MultiplyWithRoot" null (`self.VelocidadProyectilChico`) (`self.As BP Character`) null)))
    (else
      (`self.K2_DestroyActor`))))

(event `self.ReceiveTick`
  (params (DeltaSeconds :type "Float (single-precision)"))
  (`self.K2_AddActorLocalOffset` (* (`self.Velo`) (`self.Velocidad`))))

(fn `UserConstructionScript`)