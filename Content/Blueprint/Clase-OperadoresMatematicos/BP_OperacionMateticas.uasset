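; Practice actor for math operators that simulates losing health over time until it is destroyed.
; On BeginPlay, a delayed loop subtracts Daño from VidaActual via HacerDaño and prints the result with MostrarNumero every two seconds.
; Once health drops below zero, it prints a destruction message, waits briefly and destroys itself.
; An uncalled SumarDosNumeros function, a disconnected division printout and loose operator nodes remain unused.
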(event `self.ReceiveBeginPlay`
  (if (>= (`self.VidaActual`) 0.0) :!label _label
    (`self.HacerDaño` (`self.Daño`) (`self.VidaActual`))
    (`self.MostrarNumero` (`self.VidaActual`))
    (`KismetSystemLibrary.Delay` 2.0)
    (goto _label)
    (else
      (`KismetSystemLibrary.PrintString` "Te han destruido")
      (`KismetSystemLibrary.Delay` 2.0)
      (`self.K2_DestroyActor`))))

(fn `HacerDaño`
  (params (`Daño` :type "Float (double-precision)") (Vida :type "Float (double-precision)"))
  (set `self.VidaActual` (- Vida `Daño`)))

(fn `MostrarNumero`
  (params (Num :type "Float (double-precision)"))
  (`KismetSystemLibrary.PrintString` (`KismetStringLibrary.Concat_StrStr` "La vida Actaul es: \n" (`KismetStringLibrary.Conv_DoubleToString` Num)) true true (struct :`R` 0.04934 :`G` 1.0 :`B` 0.124361 :`A` 1.0) 15.0))

(fn `Sumar Dos Numeros`
  (params (N1 :type "Float (double-precision)") (N2 :type "Float (double-precision)"))
  (returns (Resultado :type "Float (double-precision)"))
  (return (+ N1 N2)))

(fn `UserConstructionScript`)