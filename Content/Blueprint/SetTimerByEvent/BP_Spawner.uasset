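; BP_Spawner is an actor that repeatedly fires BP_Proyectil1 projectiles from its own transform.
; On BeginPlay it starts a looping timer by event, using CantidaDisparossegundo directly as the interval in seconds, despite the name suggesting shots per second.
; Each tick of the timer spawns a projectile, passing VelocidadDeProyectul as its Velocidad, multiplied tenfold when the BalaRapida flag is set.
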(event `self.ReceiveBeginPlay`
  (`KismetSystemLibrary.K2_SetTimerDelegate` (delegate `SpawnearProyectil`) (`self.CantidaDisparos/segundo`) true))

(event `SpawnearProyectil`
  (if (`self.bBalaRapida`)
    (`|SpawnActorFromClass` "/Game/Blueprint/SetTimerByEvent/BP_Proyectil1.BP_Proyectil1_C" (`self.GetTransform`) "Undefined" "MultiplyWithRoot" null (* (`self.VelocidadDeProyectul`) 10.0) null)
    (else
      (`|SpawnActorFromClass` "/Game/Blueprint/SetTimerByEvent/BP_Proyectil1.BP_Proyectil1_C" (`self.GetTransform`) "Undefined" "MultiplyWithRoot" null (`self.VelocidadDeProyectul`) null))))

(fn `UserConstructionScript`)