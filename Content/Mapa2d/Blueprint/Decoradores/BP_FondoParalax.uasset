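; BP_FondoParalax is a scrolling 2D background decorator, named for parallax, built from three Paper sprites.
; Each Tick shifts all three sprites by Direccion times VelocidadScroll, without delta-time scaling, so speed depends on frame rate.
; The construction script stores the left edge of the actor bounds in Punto1, which nothing shown reads.
; Wrap-around looping and sprite-width measurement exist only as disconnected logic, so the sprites never wrap.
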(event `self.ReceiveBeginPlay`)

(event `self.ReceiveTick`
  (params (DeltaSeconds :type "Float (single-precision)"))
  (`SceneComponent.K2_AddRelativeLocation` (`self.PaperSprite1`) (* (`self.Direccion`) (`self.VelocidadScroll`)) false false)
  (`SceneComponent.K2_AddRelativeLocation` (`self.PaperSprite`) (* (`self.Direccion`) (`self.VelocidadScroll`)) false false)
  (`SceneComponent.K2_AddRelativeLocation` (`self.PaperSprite2`) (* (`self.Direccion`) (`self.VelocidadScroll`)) false false))

(fn `UserConstructionScript`
  (bind (_origin _boxextent) (`self.GetActorBounds` false true))
  (set `self.Punto1` (- (`KismetMathLibrary.MakeVector` (.x _origin) (.y _origin) (.z _origin)) (`KismetMathLibrary.MakeVector` (.x _boxextent)))))