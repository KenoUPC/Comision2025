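; BP_Nube is a decorative cloud actor for the 2D map that drifts across the world.
; On BeginPlay it picks a random speed and randomizes the Paper2D sprite's alpha while keeping its color, so clouds vary in pace and translucency.
; Each Tick offsets the actor along Direccion by that speed without sweep or delta-time scaling, so drift depends on frame rate.
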(event `self.ReceiveBeginPlay`
  (bind _papersprite (`self.PaperSprite`))
  (bind (_spritecolor_r _spritecolor_g _spritecolor_b) (break `LinearColor` (`PaperSpriteComponent.SpriteColor` _papersprite)))
  (set `self.Velocidad` (`KismetMathLibrary.RandomFloatInRange` 1.0 4.0))
  (`PaperSpriteComponent.SetSpriteColor` _papersprite (make `LinearColor` _spritecolor_r _spritecolor_g _spritecolor_b (`KismetMathLibrary.RandomFloatInRange` 0.05 0.7))))

(event `self.ReceiveTick`
  (params (DeltaSeconds :type "Float (single-precision)"))
  (`self.K2_AddActorWorldOffset` (* (`self.Direccion`) (`self.Velocidad`))))

(fn `UserConstructionScript`)