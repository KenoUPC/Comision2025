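; BP_Plataforma is an interactable platform in the 2D map that moves between points and temporarily vanishes after being touched.
; The construction script feeds two relative points into an InterpToMovement component to define its path.
; When an actor implementing BPI_Teletransportable overlaps it, a timer hides it and disables collision, then restores both after a configurable delay.
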(event `self.ReceiveBeginPlay`)

(event `self.ReceiveActorBeginOverlap`
  (params (OtherActor :type "Actor Object Reference"))
  (if (`KismetSystemLibrary.DoesImplementInterface` OtherActor "/Game/Mapa2d/BPInterface/BPI_Teletransportable.BPI_Teletransportable_C")
    (`KismetSystemLibrary.K2_SetTimerDelegate` (delegate `Desaparecer`) (`self.TiempoDestruccion`))))

(event `Desaparecer`
  (`self.SetActorHiddenInGame` true)
  (`self.SetActorEnableCollision` false)
  (`KismetSystemLibrary.Delay` (`self.TiempoDeAparicion`))
  (`self.SetActorHiddenInGame` false)
  (`self.SetActorEnableCollision` true))

(fn `UserConstructionScript`
  (bind _interptomovement (`self.InterpToMovement`))
  (`InterpToMovementComponent.AddControlPointPosition` _interptomovement (`self.Punto1`) true)
  (`InterpToMovementComponent.AddControlPointPosition` _interptomovement (`self.Punto2`) true))